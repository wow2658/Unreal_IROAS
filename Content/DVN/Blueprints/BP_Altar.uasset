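; BP_Altar is an altar prop of tree, vine and other meshes that dissolves away once the level's BP_StartTrigger is destroyed.
; One second after BeginPlay it binds to that trigger's OnDestroyed event.
; When fired, it swaps dynamic dissolve materials onto the meshes, hides its point light and drives their Dissolve parameter with a timeline.
; The actor destroys itself one second after the timeline finishes.
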(event `self.ReceiveBeginPlay`
  (`KismetSystemLibrary.Delay` 1.0)
  (bind _returnvalue (`GameplayStatics.GetActorOfClass` "/Game/YSL/Blueprints/BP_StartTrigger.BP_StartTrigger_C"))
  (add `self.OnDestroyed` _returnvalue (delegate `OnStartTriggerDestroyed`)))

(event `OnStartTriggerDestroyed` :!signature `self.OnDestroyed`
  (params (DestroyedActor :type "Actor Object Reference"))
  (bind _ww__1_ (`self.ww__1_`))
  (bind _returnvalue (`PrimitiveComponent.CreateDynamicMaterialInstance` _ww__1_ 0 "/Game/DVN/VFX/M_Dissolve_Plains_Tree_Stump01.M_Dissolve_Plains_Tree_Stump01" "None"))
  (bind _returnvalue_2 (`PrimitiveComponent.CreateDynamicMaterialInstance` _ww__1_ 1 "/Game/DVN/VFX/M_Dissolve_ChapelColumn.M_Dissolve_ChapelColumn" "None"))
  (bind _returnvalue_3 (`PrimitiveComponent.CreateDynamicMaterialInstance` (`self.SM_Plains_Vine03`) 0 "/Game/DVN/VFX/M_Dissolve_PLains_Fern01.M_Dissolve_PLains_Fern01" "None"))
  (`PrimitiveComponent.SetMaterial` (`self.SM_Plains_Tree01`) 0 _returnvalue)
  (`PrimitiveComponent.SetMaterial` (`self.ww__1_`) 0 _returnvalue)
  (`PrimitiveComponent.SetMaterial` (`self.SM_Plains_Tree_Branch03`) 0 _returnvalue)
  (`PrimitiveComponent.SetMaterial` (`self.SM_Plains_Tree_Branch01`) 0 _returnvalue)
  (`PrimitiveComponent.SetMaterial` (`self.SM_Plains_Tree03`) 0 _returnvalue)
  (`PrimitiveComponent.SetMaterial` (`self.SM_Plains_Tree_Branch02`) 0 _returnvalue)
  (`PrimitiveComponent.SetMaterial` (`self.SM_Plains_Tree02`) 0 _returnvalue)
  (`PrimitiveComponent.SetMaterial` _ww__1_ 1 _returnvalue_2)
  (`PrimitiveComponent.SetMaterial` (`self.SM_Plains_Vine02`) 0 _returnvalue_3)
  (`PrimitiveComponent.SetMaterial` (`self.SM_Plains_Vine03`) 0 _returnvalue_3)
  (`SceneComponent.SetVisibility` (`self.PointLight`) false false)
  (bind (_direction _alpha) (`Timeline|DissolveTimeline` :!via `PlayFromStart`)
    (:`Update`
      (`MaterialInstanceDynamic.SetScalarParameterValue` _returnvalue "Dissolve" _alpha)
      (`MaterialInstanceDynamic.SetScalarParameterValue` _returnvalue_2 "Dissolve" _alpha)
      (`MaterialInstanceDynamic.SetScalarParameterValue` _returnvalue_3 "Dissolve" _alpha))
    (:`Finished`
      (`KismetSystemLibrary.Delay` 1.0)
      (`self.K2_DestroyActor`))))

(fn `UserConstructionScript`)