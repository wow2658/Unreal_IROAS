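; BP_LobbyPlayerforAlpha is a lobby player Blueprint with debug hotkeys for testing ranking and leaderboard features.
; BeginPlay caches the BP_LobbyGameMode reference.
; Keys 6 and 7 submit hard-coded cleared-run records through the game mode's TestAddRanking, and key 8 calls TestGetLeaderBoard, all using a placeholder map ID.
; Key K moves the player to a fixed location without sweeping.
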(event EventBeginPlay
  (|CallParentFunction)
  (bind _asbp_lobby_game_mode (Utilities|Casting|CastToBP_LobbyGameMode (Game|GetGameMode)))
  (Variables|Default|SetLobbyGameModeRef _asbp_lobby_game_mode))

(event Collision|EventActorBeginOverlap
  (params (OtherActor :type Actor%20Object%20Reference))
  (|CallParentFunction OtherActor) ; This node is disabled and will not be called.\nDrag off pins to build functionality.
)

(event EventTick
  (params (DeltaSeconds :type Float%20%28single-precision%29))
  (|CallParentFunction DeltaSeconds) ; This node is disabled and will not be called.\nDrag off pins to build functionality.
)

(event Input|KeyboardEvents|DebugKey7
  (params (Key :type Key%20Structure) (ActionValue :type Input%20Action%20Value%20Structure))
  (:Pressed
    (Class|LobbyGameMode|TestAddRanking (Variables|Default|GetLobbyGameModeRef) "string" "2023-11-10T10:11:41.129Z" "2023-11-10T10:20:171.129Z" true)))

(event Input|KeyboardEvents|DebugKey8
  (params (Key :type Key%20Structure) (ActionValue :type Input%20Action%20Value%20Structure))
  (:Pressed
    (Class|LobbyGameMode|TestGetLeaderBoard (Variables|Default|GetLobbyGameModeRef) "string")))

(event Input|KeyboardEvents|DebugKey6
  (params (Key :type Key%20Structure) (ActionValue :type Input%20Action%20Value%20Structure))
  (:Pressed
    (Class|LobbyGameMode|TestAddRanking (Variables|Default|GetLobbyGameModeRef) "string" "2023-11-10T08:35:41.129Z" "2023-11-10T08:47:41.129Z" true)))

(event Input|KeyboardEvents|DebugKeyK
  (params (Key :type Key%20Structure) (ActionValue :type Input%20Action%20Value%20Structure))
  (:Pressed
    (Transformation|SetActorLocation "2551.000000,3730.000000,233.000000" false false)))

(fn ConstructionScript
  (|CallParentFunction))