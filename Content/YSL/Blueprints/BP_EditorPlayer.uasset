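; BP_EditorPlayer is an editor player Blueprint that currently holds only debug test logic.
; Pressing a debug S key creates a dynamic instance of the M_Select material and sets its StencilValue negative, and releasing flips it positive, printing the value each time.
; The left thumbstick edit Enhanced Input action only prints its value.
; An EditorZoomSpline actor lookup is unconnected and never runs.
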(event Input|EnhancedActionEvents|EnhancedInputActionIA_ThumbstickAxisLeft
  (params (ActionValue :type Vector%202D%20Structure) (ElapsedSeconds :type Float%20%28double-precision%29) (TriggeredSeconds :type Float%20%28double-precision%29) (InputAction :type Input%20Action%20Object%20Reference :default "/Game/DVN/Input/InputActions/IA_ThumbstickAxisLeft.IA_ThumbstickAxisLeft")))

(event Input|EnhancedActionEvents|EnhancedInputActionIA_ThumbstickAxisLeft_Edit
  (params (ActionValue :type Float%20%28double-precision%29) (ElapsedSeconds :type Float%20%28double-precision%29) (TriggeredSeconds :type Float%20%28double-precision%29) (InputAction :type Input%20Action%20Object%20Reference :default "/Game/YSL/Inputs/InputActions/IA_ThumbstickAxisLeft_Edit.IA_ThumbstickAxisLeft_Edit")))

(event Input|EnhancedActionEvents|EnhancedInputActionIA_LThumbstickLeft_Edit
  (params (ActionValue :type Boolean) (ElapsedSeconds :type Float%20%28double-precision%29) (TriggeredSeconds :type Float%20%28double-precision%29) (InputAction :type Input%20Action%20Object%20Reference :default "/Game/YSL/Inputs/InputActions/IA_LThumbstickLeft_Edit.IA_LThumbstickLeft_Edit"))
  (:Triggered
    (Development|PrintString (Utilities|String|ToString(Boolean) ActionValue))))

(event EventBeginPlay)

(event Collision|EventActorBeginOverlap
  (params (OtherActor :type Actor%20Object%20Reference)))

(event EventTick
  (params (DeltaSeconds :type Float%20%28single-precision%29)))

(event Input|KeyboardEvents|DebugKeyS
  (params (Key :type Key%20Structure :default "None") (ActionValue :type Input%20Action%20Value%20Structure))
  (:Pressed
    (bind _returnvalue (Rendering|Material|CreateDynamicMaterialInstance "/Game/YSL/Mat/M_Select.M_Select" "None" "None" :!class /Script/Engine.KismetMaterialLibrary))
    (bind _output_get (Variables|Default|SetNewVar _returnvalue))
    (Rendering|Material|SetScalarParameterValue _output_get "StencilValue" -1.0 :!class /Script/Engine.MaterialInstanceDynamic)
    (bind _returnvalue_2 (Rendering|Material|GetScalarParameterValue _output_get "StencilValue" :!class /Script/Engine.MaterialInstanceDynamic))
    (Development|PrintString (Utilities|String|ToString(Float) _returnvalue_2)))
  (:Released
    (Rendering|Material|SetScalarParameterValue _output_get "StencilValue" 1.0 :!class /Script/Engine.MaterialInstanceDynamic)
    (bind _returnvalue_3 (Rendering|Material|GetScalarParameterValue _output_get "StencilValue" :!class /Script/Engine.MaterialInstanceDynamic))
    (Development|PrintString (Utilities|String|ToString(Float) _returnvalue_3))))

(fn ConstructionScript)